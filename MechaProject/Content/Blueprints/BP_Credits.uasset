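; Credits Blueprint that shows the WBP_Credits widget on BeginPlay and also carries a player respawn loop.
; Respawn binds Death to the first-person character's OnDestroyed event.
; After a short delay, Death spawns a new character at SpawnLocation, possesses it and calls Respawn to rebind.
; BeginPlay does not call Respawn, so nothing in this graph starts that loop.
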(event Custom|Death
  (params (DestroyedActor :type Actor%20Object%20Reference))
  (Utilities|FlowControl|Delay 1.5)
  (bind _returnvalue (Game|SpawnActorfromClass "/Game/FirstPerson/Blueprints/BP_FirstPersonCharacter.BP_FirstPersonCharacter_C" (Variables|Default|GetSpawn%20Location) "AdjustIfPossibleButAlwaysSpawn" 0 0))
  (Pawn|Possess (Game|GetPlayerController 0) _returnvalue)
  (CallFunction|Respawn))

(event Custom|Respawn
  (bind _asbp_first_person_character (Utilities|Casting|CastToBP_FirstPersonCharacter (Game|GetPlayerCharacter 0)))
  (Game|BindEventtoOnDestroyed _asbp_first_person_character (delegate Custom|Death)))

(event EventBeginPlay
  (bind _returnvalue (UserInterface|CreateWidget "/Game/UI/WBP_Credits.WBP_Credits_C"))
  (UserInterface|Viewport|AddtoViewport _returnvalue 0))

(event EventTick
  (params (DeltaSeconds :type Float%20%28single-precision%29)))

(fn ConstructionScript
  (|CallParentFunction))